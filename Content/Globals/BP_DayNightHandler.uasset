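; Day/night cycle actor that drives the game clock and sun, registering itself with the game instance.
; A looping timeline rotates the directional light and writes time and day to the game instance, with each cycle starting at 06:00.
; Wait fast-forwards the timeline to a target time, handling wraparound, then notifies its invoker.
; Each cycle end increments the day and resets the wagon if at market.
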(event Custom|PauseTime
  (bind _gameinstanceref (Variables|Default|GetGameInstanceRef))
  (bind _lerp (Timeline|Timeline Stop)
    (:Update
      (Transformation|SetActorRotation (Variables|Default|GetsunlightRef) (Math|Rotator|Lerp(Rotator) "0.000000,180.000000,0.000000" "-359.000000,180.000000,0.000000" _lerp))
      (Variables|/Game/Globals/BP_GameInstance.BP_GameInstance_C|SetgameTime _gameinstanceref (Utilities|Struct|MakeDS_GameTime (.hours (Math|Timespan|MakeTimespan 0 6 0 (Math|Float|Truncate (Math|Float|Lerp 0.0 8.64e+04 _lerp)))) (.minutes (Math|Timespan|MakeTimespan 0 6 0 (Math|Float|Truncate (Math|Float|Lerp 0.0 8.64e+04 _lerp)))) (.seconds (Math|Timespan|MakeTimespan 0 6 0 (Math|Float|Truncate (Math|Float|Lerp 0.0 8.64e+04 _lerp))))))
      (Variables|/Game/Globals/BP_GameInstance.BP_GameInstance_C|SetgameDay _gameinstanceref (.days (Math|Timespan|MakeTimespan 0 6 0 (Math|Float|Truncate (Math|Float|Lerp 0.0 8.64e+04 _lerp)))))
      (if (and (Variables|Default|Getwaiting) (Variables|Default|GetwaitHasLooped))
        (if (>= (Components|Timeline|GetPlaybackPosition (Variables|Default|GetTimeline)) (Variables|Default|GetwaitTarget))
          (CallFunction|FInishWaiting))))
    (:Finished
      (Math|Integer|IncrementInt (Variables|/Game/Globals/BP_GameInstance.BP_GameInstance_C|GetgameDay (Variables|Default|GetGameInstanceRef))
        (:%20%20
          (if (Variables|Default|Getwaiting)
            (if (Variables|Default|GetwaitHasLooped)
              (Development|PrintString "somethings gone fucky")
              (else
                (Variables|Default|SetwaitHasLooped true))))
          (bind _returnvalue (Actor|GetActorOfClass "/Game/Objects/BP_Wagon.BP_Wagon_C"))
          (if (Variables|/Game/Objects/BP_Wagon.BP_Wagon_C|GetcartAtMarket _returnvalue)
            (Default|ResetWagon _returnvalue)
            (Timeline|Timeline PlayFromStart)
            (else
              (Timeline|Timeline PlayFromStart))))))))

(event Custom|RestartDayNightCycle
  (bind _gameinstanceref (Variables|Default|GetGameInstanceRef))
  (bind _lerp (Timeline|Timeline PlayFromStart)
    (:Update
      (Transformation|SetActorRotation (Variables|Default|GetsunlightRef) (Math|Rotator|Lerp(Rotator) "0.000000,180.000000,0.000000" "-359.000000,180.000000,0.000000" _lerp))
      (Variables|/Game/Globals/BP_GameInstance.BP_GameInstance_C|SetgameTime _gameinstanceref (Utilities|Struct|MakeDS_GameTime (.hours (Math|Timespan|MakeTimespan 0 6 0 (Math|Float|Truncate (Math|Float|Lerp 0.0 8.64e+04 _lerp)))) (.minutes (Math|Timespan|MakeTimespan 0 6 0 (Math|Float|Truncate (Math|Float|Lerp 0.0 8.64e+04 _lerp)))) (.seconds (Math|Timespan|MakeTimespan 0 6 0 (Math|Float|Truncate (Math|Float|Lerp 0.0 8.64e+04 _lerp))))))
      (Variables|/Game/Globals/BP_GameInstance.BP_GameInstance_C|SetgameDay _gameinstanceref (.days (Math|Timespan|MakeTimespan 0 6 0 (Math|Float|Truncate (Math|Float|Lerp 0.0 8.64e+04 _lerp)))))
      (if (and (Variables|Default|Getwaiting) (Variables|Default|GetwaitHasLooped))
        (if (>= (Components|Timeline|GetPlaybackPosition (Variables|Default|GetTimeline)) (Variables|Default|GetwaitTarget))
          (CallFunction|FInishWaiting))))
    (:Finished
      (Math|Integer|IncrementInt (Variables|/Game/Globals/BP_GameInstance.BP_GameInstance_C|GetgameDay (Variables|Default|GetGameInstanceRef))
        (:%20%20
          (if (Variables|Default|Getwaiting)
            (if (Variables|Default|GetwaitHasLooped)
              (Development|PrintString "somethings gone fucky")
              (else
                (Variables|Default|SetwaitHasLooped true))))
          (bind _returnvalue (Actor|GetActorOfClass "/Game/Objects/BP_Wagon.BP_Wagon_C"))
          (if (Variables|/Game/Objects/BP_Wagon.BP_Wagon_C|GetcartAtMarket _returnvalue)
            (Default|ResetWagon _returnvalue)
            (Timeline|Timeline PlayFromStart)
            (else
              (Timeline|Timeline PlayFromStart))))))))

(event Custom|SetTime
  (params (newTime :type Float%20%28double-precision%29))
  (bind _gameinstanceref (Variables|Default|GetGameInstanceRef))
  (bind _lerp (Timeline|Timeline SetNewTime)
    (:Update
      (Transformation|SetActorRotation (Variables|Default|GetsunlightRef) (Math|Rotator|Lerp(Rotator) "0.000000,180.000000,0.000000" "-359.000000,180.000000,0.000000" _lerp))
      (Variables|/Game/Globals/BP_GameInstance.BP_GameInstance_C|SetgameTime _gameinstanceref (Utilities|Struct|MakeDS_GameTime (.hours (Math|Timespan|MakeTimespan 0 6 0 (Math|Float|Truncate (Math|Float|Lerp 0.0 8.64e+04 _lerp)))) (.minutes (Math|Timespan|MakeTimespan 0 6 0 (Math|Float|Truncate (Math|Float|Lerp 0.0 8.64e+04 _lerp)))) (.seconds (Math|Timespan|MakeTimespan 0 6 0 (Math|Float|Truncate (Math|Float|Lerp 0.0 8.64e+04 _lerp))))))
      (Variables|/Game/Globals/BP_GameInstance.BP_GameInstance_C|SetgameDay _gameinstanceref (.days (Math|Timespan|MakeTimespan 0 6 0 (Math|Float|Truncate (Math|Float|Lerp 0.0 8.64e+04 _lerp)))))
      (if (and (Variables|Default|Getwaiting) (Variables|Default|GetwaitHasLooped))
        (if (>= (Components|Timeline|GetPlaybackPosition (Variables|Default|GetTimeline)) (Variables|Default|GetwaitTarget))
          (CallFunction|FInishWaiting))))
    (:Finished
      (Math|Integer|IncrementInt (Variables|/Game/Globals/BP_GameInstance.BP_GameInstance_C|GetgameDay (Variables|Default|GetGameInstanceRef))
        (:%20%20
          (if (Variables|Default|Getwaiting)
            (if (Variables|Default|GetwaitHasLooped)
              (Development|PrintString "somethings gone fucky")
              (else
                (Variables|Default|SetwaitHasLooped true))))
          (bind _returnvalue (Actor|GetActorOfClass "/Game/Objects/BP_Wagon.BP_Wagon_C"))
          (if (Variables|/Game/Objects/BP_Wagon.BP_Wagon_C|GetcartAtMarket _returnvalue)
            (Default|ResetWagon _returnvalue)
            (Timeline|Timeline PlayFromStart)
            (else
              (Timeline|Timeline PlayFromStart))))))))

(event Custom|ResumeTime
  (bind _gameinstanceref (Variables|Default|GetGameInstanceRef))
  (bind _lerp (Timeline|Timeline Play)
    (:Update
      (Transformation|SetActorRotation (Variables|Default|GetsunlightRef) (Math|Rotator|Lerp(Rotator) "0.000000,180.000000,0.000000" "-359.000000,180.000000,0.000000" _lerp))
      (Variables|/Game/Globals/BP_GameInstance.BP_GameInstance_C|SetgameTime _gameinstanceref (Utilities|Struct|MakeDS_GameTime (.hours (Math|Timespan|MakeTimespan 0 6 0 (Math|Float|Truncate (Math|Float|Lerp 0.0 8.64e+04 _lerp)))) (.minutes (Math|Timespan|MakeTimespan 0 6 0 (Math|Float|Truncate (Math|Float|Lerp 0.0 8.64e+04 _lerp)))) (.seconds (Math|Timespan|MakeTimespan 0 6 0 (Math|Float|Truncate (Math|Float|Lerp 0.0 8.64e+04 _lerp))))))
      (Variables|/Game/Globals/BP_GameInstance.BP_GameInstance_C|SetgameDay _gameinstanceref (.days (Math|Timespan|MakeTimespan 0 6 0 (Math|Float|Truncate (Math|Float|Lerp 0.0 8.64e+04 _lerp)))))
      (if (and (Variables|Default|Getwaiting) (Variables|Default|GetwaitHasLooped))
        (if (>= (Components|Timeline|GetPlaybackPosition (Variables|Default|GetTimeline)) (Variables|Default|GetwaitTarget))
          (CallFunction|FInishWaiting))))
    (:Finished
      (Math|Integer|IncrementInt (Variables|/Game/Globals/BP_GameInstance.BP_GameInstance_C|GetgameDay (Variables|Default|GetGameInstanceRef))
        (:%20%20
          (if (Variables|Default|Getwaiting)
            (if (Variables|Default|GetwaitHasLooped)
              (Development|PrintString "somethings gone fucky")
              (else
                (Variables|Default|SetwaitHasLooped true))))
          (bind _returnvalue (Actor|GetActorOfClass "/Game/Objects/BP_Wagon.BP_Wagon_C"))
          (if (Variables|/Game/Objects/BP_Wagon.BP_Wagon_C|GetcartAtMarket _returnvalue)
            (Default|ResetWagon _returnvalue)
            (Timeline|Timeline PlayFromStart)
            (else
              (Timeline|Timeline PlayFromStart))))))))

(event Custom|Wait
  (params (GameHoursToWait :type Integer) (waitInvoker :type BP%20Bed%20Object%20Reference))
  (bind _returnvalue (* GameHoursToWait 60 60))
  (bind _timeline (Variables|Default|GetTimeline))
  (bind _returnvalue_2 (Components|Timeline|GetPlaybackPosition _timeline))
  (bind _returnvalue_3 (/ _returnvalue 12))
  (bind _returnvalue_4 (+ _returnvalue_2 _returnvalue_3))
  (Variables|Default|SetwaitInvoker waitInvoker)
  (if (== GameHoursToWait 0)
    (CallFunction|FInishWaiting)
    (else
      (if (> _returnvalue_4 7.2e+03)
        (Variables|Default|SetwaitTarget (- _returnvalue_4 7.2e+03))
        (Variables|Default|SetwaitHasLooped false)
        (else
          (Variables|Default|SetwaitTarget _returnvalue_4)
          (Variables|Default|SetwaitHasLooped true)))
      (Variables|Default|Setwaiting true)
      (Components|Timeline|SetPlayRate _timeline 2e+02)
      (CallFunction|ResumeTime))))

(event Custom|FInishWaiting
  (CallFunction|PauseTime)
  (Components|Timeline|SetPlayRate (Variables|Default|GetTimeline) 1.0)
  (CallFunction|ResumeTime)
  (Default|CompleteRest (Variables|Default|GetwaitInvoker)))

(event EventBeginPlay
  (Variables|Default|SetGameInstanceRef (.AsBP%20Game%20Instance (Utilities|Casting|CastToBP_GameInstance (Game|GetGameInstance))))
  (bind _returnvalue (Actor|GetActorOfClass "/Script/Engine.DirectionalLight"))
  (Variables|Default|SetsunlightRef _returnvalue)
  (CallFunction|RestartDayNightCycle)
  (Variables|/Game/Globals/BP_GameInstance.BP_GameInstance_C|SetdayNightHandler (Variables|Default|GetGameInstanceRef) self))

(event Collision|EventActorBeginOverlap
  (params (OtherActor :type Actor%20Object%20Reference)))

(event EventTick
  (params (DeltaSeconds :type Float%20%28single-precision%29)))

(fn ConstructionScript)