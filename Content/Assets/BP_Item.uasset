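; BP_Item is an interactable pickup actor that the player can take into an empty held-item slot.
; On BeginPlay it builds the name in its interaction data from the SelfObjectType class defaults, formatted as "type of variant", and GetInfo returns that data.
; Interact stores SelfObjectType as the player's HeldItemData if none is held, shows the SmallHeldItem component and destroys the actor.
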(event EventBeginPlay
  (bind _self_objecttype (Variables|Default|Getself_ObjectType))
  (bind (_singularitemtype _selftype) (Utilities|GetClassDefaults _self_objecttype))
  (Utilities|Struct|SetmembersinDS_InteractionData (Variables|Default|GetSelfData) (Utilities|Text|FormatText "{Type} of {Var}" _singularitemtype _selftype)))

(event Collision|EventActorBeginOverlap
  (params (OtherActor :type Actor%20Object%20Reference)))

(event EventTick
  (params (DeltaSeconds :type Float%20%28single-precision%29)))

(event EventInteract
  (params (playerRef :type BP%20Player%20Object%20Reference))
  (if (not (Utilities|IsValidClass (Variables|/Game/FirstPerson/Blueprints/BP_Player.BP_Player_C|GetheldItemData playerRef)))
    (Variables|/Game/FirstPerson/Blueprints/BP_Player.BP_Player_C|SetheldItemData playerRef (Variables|Default|GetSelf_ObjectType))
    (Rendering|SetVisibility (Variables|/Game/FirstPerson/Blueprints/BP_Player.BP_Player_C|GetSmallHeldItem playerRef) true false)
    (Actor|DestroyActor)))

(fn ConstructionScript)

(fn GetInfo
  (return (Variables|Default|GetSelfData)))