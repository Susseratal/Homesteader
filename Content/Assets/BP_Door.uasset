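; BP_Door is an interactable door that the player toggles between open and closed.
; Interact instantly snaps the door mesh between zero and 90-degree relative rotation, flips the open flag, then reruns OnObserved.
; OnObserved sets the interaction data's verb according to the open state and sends it to the observer's prompt.
; GetInfo returns that same interaction data.
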(event EventBeginPlay)

(event Collision|EventActorBeginOverlap
  (params (OtherActor :type Actor%20Object%20Reference)))

(event EventTick
  (params (DeltaSeconds :type Float%20%28single-precision%29)))

(event EventOnObserved
  (params (Observer :type BP%20Player%20Object%20Reference))
  (if (Variables|Default|Getb_open)
    (bind _structout (Utilities|Struct|SetmembersinDS_InteractionData (Variables|Default|GetSelfData) (Utilities|Array|MakeArray "NewEnumerator7")))
    (Variables|Default|SetSelfData _structout)
    (else
      (bind _structout_2 (Utilities|Struct|SetmembersinDS_InteractionData (Variables|Default|GetSelfData) (Utilities|Array|MakeArray "NewEnumerator6")))
      (Variables|Default|SetSelfData _structout_2)))
  (Default|SetPromptInfo Observer (Variables|Default|GetSelfData)))

(event EventInteract
  (params (playerRef :type BP%20Player%20Object%20Reference))
  (bind _doormesh (Variables|Default|GetDoorMesh))
  (if (Variables|Default|Getb_open)
    (Transformation|SetRelativeRotation _doormesh "0, 0, 0" false false)
    (else
      (Transformation|SetRelativeRotation _doormesh "0.000000,90.000000,0.000000" false false)))
  (Variables|Default|Setb_open (not (Variables|Default|Getb_open)))
  (CallFunction|OnObserved playerRef))

(fn ConstructionScript)

(fn GetInfo
  (return (Variables|Default|GetSelfData)))