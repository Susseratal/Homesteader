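; Interactable item generator that accumulates produce for the player to pick up one at a time when empty-handed.
; The SelfProducer class defaults drive its mesh, name, label placement, interval and odds.
; Tick runs a Delay scaled by frame delta and the game instance's day/night rest multiplier, then a random gate adds rest-scaled produce and updates the text.
; Observers get a HUD prompt with an extra verb when holding grain, though secondary interaction does nothing yet.
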(event EventBeginPlay)

(event Collision|EventActorBeginOverlap
  (params (OtherActor :type Actor%20Object%20Reference)))

(event EventTick
  (params (DeltaSeconds :type Float%20%28single-precision%29))
  (bind _returnvalue (Game|GetGameInstance))
  (bind _selfproducer (Variables|Default|GetselfProducer))
  (bind _asbp_game_instance (Utilities|Casting|CastToBP_GameInstance _returnvalue))
  (bind _generatorvalues (Utilities|GetClassDefaults _selfproducer))
  (bind (_interval _randomnessrange _randomnessgate) (Utilities|Struct|BreakDS_GenerationValues _generatorvalues))
  (bind _daynighthandler (Variables|/Game/Globals/BP_GameInstance.BP_GameInstance_C|GetdayNightHandler _asbp_game_instance))
  (bind (_x _y) (Utilities|Struct|BreakIntVector2d _randomnessrange))
  (Utilities|FlowControl|Delay (* DeltaSeconds (* _interval (Variables|/Game/Globals/BP_DayNightHandler.BP_DayNightHandler_C|GetrestIntervalMultiplier _daynighthandler))))
  (if (== (Math|Random|RandomIntegerinRange _x _y) _randomnessgate)
    (Variables|Default|SetproduceQuantity (+ (Variables|Default|GetproduceQuantity) (Variables|/Game/Globals/BP_DayNightHandler.BP_DayNightHandler_C|GetrestMultiplier _daynighthandler)))
    (CallFunction|UpdateText)))

(event EventOnObserved
  (params (Observer :type BP%20Player%20Object%20Reference))
  (bind _selfdata (Variables|Default|GetselfData))
  (if (Default|IsPlayerHoldingSomething Observer)
    (if (== (Variables|/Game/FirstPerson/Blueprints/BP_Player.BP_Player_C|GetheldItemData Observer) "/Game/Assets/ObjectData/DBP_Grain.DBP_Grain_C")
      (Utilities|Struct|SetmembersinDS_InteractionData _selfdata (Utilities|Array|MakeArray "NewEnumerator12" "NewEnumerator13"))
      (else
        (Utilities|Struct|SetmembersinDS_InteractionData _selfdata (Utilities|Array|MakeArray "NewEnumerator12") :!label _label)))
    (else
      (goto _label)))
  (Default|SetPromptData (Variables|/Game/FirstPerson/Blueprints/BP_Player.BP_Player_C|GetW_HudRef Observer) (Variables|Default|GetselfData)))

(event EventSecondaryInteract
  (params (Instigator :type BP%20Player%20Object%20Reference))
  (if (Default|IsPlayerHoldingSomething Instigator)
    (if (== (Variables|/Game/FirstPerson/Blueprints/BP_Player.BP_Player_C|GetheldItemData Instigator) "/Game/Assets/ObjectData/DBP_Grain.DBP_Grain_C")
      _)))

(event EventInteract
  (params (playerRef :type BP%20Player%20Object%20Reference))
  (if (and (not (Default|IsPlayerHoldingSomething playerRef)) (> (Variables|Default|GetproduceQuantity) 0))
    (Variables|/Game/FirstPerson/Blueprints/BP_Player.BP_Player_C|SetheldItemData playerRef (Variables|Default|GetselfProducer))
    (Rendering|SetVisibility (Variables|/Game/FirstPerson/Blueprints/BP_Player.BP_Player_C|GetSmallHeldItem playerRef) true false)
    (Math|Integer|DecrementInt (Variables|Default|GetproduceQuantity)
      (:%20%20
        (CallFunction|UpdateText)))))

(fn ConstructionScript
  (bind _selfproducer (Variables|Default|GetselfProducer))
  (bind (_singularitemtype _selftype _itemvalue _generatormesh _generatorname _generatorvalues _generatorresourcecost _textrenderlocation) (Utilities|GetClassDefaults _selfproducer))
  (Components|StaticMesh|SetStaticMesh (Variables|Default|GetCube) _generatormesh)
  (Variables|Default|SetselfData (Utilities|Struct|MakeDS_InteractionData _generatorname (Utilities|Array|MakeArray "NewEnumerator12")))
  (Transformation|SetRelativeLocation (Variables|Default|GetTextRender) _textrenderlocation false false))

(fn UpdateText
  (Rendering|Components|TextRender|SetText (Variables|Default|GetTextRender) (Utilities|Text|FormatText "{x} {y}" (Variables|Default|GetproduceQuantity) (.SelfType (Utilities|GetClassDefaults (Variables|Default|GetselfProducer))))))

(fn GetInfo
  (return (Variables|Default|GetselfData)))