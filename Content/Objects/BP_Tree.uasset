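; BP_Tree is a choppable tree that can be felled for logs and later restored.
; DespawnTree marks it chopped, hides it, disables mesh collision and spawns BP_Logs slightly above its location.
; RespawnTree reverses this only if it was chopped, restoring visibility and collision on the same actor rather than spawning a new one.
; GetInfo returns interaction data naming it "Tree"; the event graph has no active logic.
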(event EventBeginPlay)

(event Collision|EventActorBeginOverlap
  (params (OtherActor :type Actor%20Object%20Reference)))

(event EventTick
  (params (DeltaSeconds :type Float%20%28single-precision%29)))

(fn ConstructionScript)

(fn DespawnTree
  (bind _defaultsceneroot (Variables|Default|GetDefaultSceneRoot))
  (bind _returnvalue (Transformation|GetWorldLocation _defaultsceneroot))
  (Variables|Default|Setchopped true)
  (Rendering|SetVisibility (Variables|Default|GetDefaultSceneRoot) false true)
  (Collision|SetCollisionEnabled (Variables|Default|GetTreeMesh) "NoCollision")
  (Game|SpawnActorfromClass "/Game/Objects/BP_Logs.BP_Logs_C" (Math|Transform|MakeTransform (Math|Vector|MakeVector (.x _returnvalue) (.y _returnvalue) (+ (.z _returnvalue) 5e+01)) "0, 0, 0" "1.000000,1.000000,1.000000") "Undefined" "MultiplyWithRoot" 0 0))

(fn RespawnTree
  (if (Variables|Default|Getchopped)
    (Variables|Default|Setchopped false)
    (Rendering|SetVisibility (Variables|Default|GetDefaultSceneRoot) true true)
    (Collision|SetCollisionEnabled (Variables|Default|GetTreeMesh) "QueryAndPhysics")))

(fn GetInfo
  (return (Utilities|Struct|MakeDS_InteractionData "Tree" "NewEnumerator4")))