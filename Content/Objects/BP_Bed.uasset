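; BP_Bed is an interactable bed that lets the player wait a chosen number of in-game hours.
; Interact pauses time through the GameInstance's DayNightHandler and shows the HUD wait-time slider, passing itself as BedHandle.
; ConfirmWait asks the handler to wait those hours with the bed as invoker, and CompleteRest hides and resets the slider.
; GetInfo supplies its name and interaction verb.
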(event Custom|CompleteRest
  (Default|ToggleWaitTimeSlider (Variables|/Game/FirstPerson/Blueprints/BP_Player.BP_Player_C|GetW_HudRef (Variables|Default|GetplayerHandle)) "Hidden")
  (Class|Slider|SetValue (Variables|/Game/UserInterface/W_HUD.W_HUD_C|GetSlider_52 (Variables|/Game/FirstPerson/Blueprints/BP_Player.BP_Player_C|GetW_HudRef (stale EventInteract playerRef))) 0.0))

(event Custom|ConfirmWait
  (params (hoursToWait :type Integer))
  (Default|Wait (Variables|/Game/Globals/BP_GameInstance.BP_GameInstance_C|GetdayNightHandler (.AsBP%20Game%20Instance (Utilities|Casting|CastToBP_GameInstance (Game|GetGameInstance)))) hoursToWait self))

(event EventBeginPlay)

(event Collision|EventActorBeginOverlap
  (params (OtherActor :type Actor%20Object%20Reference)))

(event EventTick
  (params (DeltaSeconds :type Float%20%28single-precision%29)))

(event EventInteract
  (params (playerRef :type BP%20Player%20Object%20Reference))
  (bind _w_hudref (Variables|/Game/FirstPerson/Blueprints/BP_Player.BP_Player_C|GetW_HudRef playerRef))
  (Variables|Default|SetplayerHandle playerRef)
  (Default|PauseTime (Variables|/Game/Globals/BP_GameInstance.BP_GameInstance_C|GetdayNightHandler (.AsBP%20Game%20Instance (Utilities|Casting|CastToBP_GameInstance (Game|GetGameInstance)))))
  (Variables|/Game/UserInterface/W_HUD.W_HUD_C|SetbedHandle _w_hudref self)
  (Default|ToggleWaitTimeSlider _w_hudref "Visible"))

(fn ConstructionScript)

(fn GetInfo
  (return (Utilities|Struct|MakeDS_InteractionData "Bed" (Utilities|Array|MakeArray "NewEnumerator11"))))