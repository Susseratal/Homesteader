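; BP_WagonHatch is an interactable wagon hatch that the player toggles open and closed.
; Interact snaps the static mesh between two relative rotations with no animation and flips BOpen.
; It then calls OnObserved, which sets the verb in SelfData to match the open state and pushes it to the observer's prompt.
; GetInfo returns that interaction data.
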(event EventBeginPlay)

(event Collision|EventActorBeginOverlap
  (params (OtherActor :type Actor%20Object%20Reference)))

(event EventTick
  (params (DeltaSeconds :type Float%20%28single-precision%29)))

(event EventOnObserved
  (params (Observer :type BP%20Player%20Object%20Reference))
  (bind _selfdata (Variables|Default|GetSelfData))
  (if (Variables|Default|Getb_open)
    (Utilities|Struct|SetmembersinDS_InteractionData _selfdata (Utilities|Array|MakeArray "NewEnumerator7"))
    (else
      (Utilities|Struct|SetmembersinDS_InteractionData _selfdata (Utilities|Array|MakeArray "NewEnumerator6"))))
  (Default|SetPromptInfo Observer (Variables|Default|GetSelfData)))

(event EventInteract
  (params (playerRef :type BP%20Player%20Object%20Reference))
  (bind _staticmesh (Variables|Default|GetStaticMesh))
  (if (Variables|Default|Getb_open)
    (Transformation|SetRelativeRotation _staticmesh "0, 0, 0" false false)
    (else
      (Transformation|SetRelativeRotation _staticmesh "0.000000,0.000000,-150.000000" false false)))
  (Variables|Default|Setb_open (not (Variables|Default|Getb_open)))
  (CallFunction|OnObserved playerRef))

(fn ConstructionScript)

(fn GetInfo
  (return (Variables|Default|GetSelfData)))