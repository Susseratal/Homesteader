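; BP_Wagon is a wagon actor with a chair and a crate container, set up for trips to market.
; On BeginPlay it passes itself to its BP_WagonChair child actor as that chair's WagonHandle.
; LeaveForMarket takes a player handle and loops over crates overlapping the Container, but the loop body is empty and the crate Value read is unconnected.
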(event Custom|LeaveForMarket
  (params (playerHandle :type BP%20Player%20Object%20Reference))
  (for _array_element (Collision|GetOverlappingActors (Variables|Default|GetContainer) "/Game/Assets/BP_Crate.BP_Crate_C" :!class /Script/Engine.PrimitiveComponent)
    _))

(event EventBeginPlay
  (Variables|/Game/Objects/BP_WagonChair.BP_WagonChair_C|SetwagonHandle (.AsBP%20Wagon%20Chair (Utilities|Casting|CastToBP_WagonChair (Variables|/Script/Engine.ChildActorComponent|GetChildActor (Variables|Default|GetWagonChair)))) self))

(event Collision|EventActorBeginOverlap
  (params (OtherActor :type Actor%20Object%20Reference)))

(event EventTick
  (params (DeltaSeconds :type Float%20%28single-precision%29)))

(fn ConstructionScript)