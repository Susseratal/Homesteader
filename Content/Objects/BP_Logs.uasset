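; BP_Logs is a physics-simulated log pickup that the player collects through interaction.
; GetInfo supplies the interaction data, naming it Logs with a single verb.
; On Interact it increments the player's Logs count, calls CheckBuildState on the player, then destroys itself.
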(event EventBeginPlay
  (Physics|SetSimulatePhysics (Variables|Default|GetSM_Logs) true))

(event Collision|EventActorBeginOverlap
  (params (OtherActor :type Actor%20Object%20Reference)))

(event EventTick
  (params (DeltaSeconds :type Float%20%28single-precision%29)))

(event EventInteract
  (params (playerRef :type BP%20Player%20Object%20Reference))
  (Math|Integer|IncrementInt (Variables|/Game/FirstPerson/Blueprints/BP_Player.BP_Player_C|Getlogs playerRef)
    (:%20%20
      (Default|CheckBuildState playerRef)
      (Actor|DestroyActor))))

(fn ConstructionScript)

(fn GetInfo
  (return (Utilities|Struct|MakeDS_InteractionData "Logs" (Utilities|Array|MakeArray "NewEnumerator0"))))